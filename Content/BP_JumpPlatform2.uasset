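; BP_JumpPlatform2 is a jump pad that launches the player character along its Arrow component's forward direction.
; On actor overlap it calls 플레이어감지 (player detection), then 튀어오르기 (bounce).
; The bounce applies a velocity-change impulse to player 0's CharacterMovement, scaled by 점프력 (jump force).
; The player check's branch is empty, so any overlapping actor triggers the launch of player 0.
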(event EventBeginPlay)

(event Collision|EventActorBeginOverlap
  (params (OtherActor :type Actor%20Object%20Reference))
  (CallFunction|플레이어감지 OtherActor)
  (CallFunction|튀어오르기))

(event EventTick
  (params (DeltaSeconds :type Float%20%28single-precision%29)))

(fn ConstructionScript)

(fn 플레이어감지
  (params (B :type Object%20Object%20Reference))
  (if (== (Game|GetPlayerCharacter 0) B)
    _))

(fn 튀어오르기
  (Physics|AddImpulse (Variables|/Script/Engine.Character|GetCharacterMovement (Game|GetPlayerCharacter 0)) (* (Math|Vector|GetForwardVector (Variables|Default|GetArrow)) (Variables|Default|Get점프력)) true))