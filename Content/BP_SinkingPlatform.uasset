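; BP_SinkingPlatform is a platform that moves away when any actor overlaps it, then returns after a delay.
; The Blocksinking timeline lerps Box's relative location from origin to the 이동방향 offset, guarded by the 내려감 flag.
; A four-second Delay chained to that timeline's Update starts Blockfloating, which lerps Box back.
; Blockfloating clears the flag on Update, so retriggering is possible before the return finishes.
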(event EventBeginPlay)

(event EventTick
  (params (DeltaSeconds :type Float%20%28single-precision%29)))

(event Collision|EventActorBeginOverlap
  (params (OtherActor :type Actor%20Object%20Reference))
  (if (not (Variables|false|Get내려감))
    (Variables|false|Set내려감 true)
    (bind _새_트랙_0 (Timeline|blocksinking PlayFromStart)
      (:Update
        (Transformation|SetRelativeLocation (Variables|Default|GetBox) (Math|Vector|Lerp(Vector) "0, 0, 0" (Variables|디폴트|Get이동방향) _새_트랙_0) false false)
        (Utilities|FlowControl|Delay 4.0)
        (bind _새_트랙_0_2 (Timeline|blockfloating PlayFromStart)
          (:Update
            (Transformation|SetRelativeLocation (Variables|Default|GetBox) (Math|Vector|Lerp(Vector) (Variables|디폴트|Get이동방향) "0, 0, 0" _새_트랙_0_2) false false)
            (Variables|false|Set내려감 false)))))))

(fn ConstructionScript)