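; Checkpoint actor with two trigger boxes, where Box2 is meant to launch the player character upward.
; Box sets the 체크도달 (checkpoint reached) flag, but BeginPlay already sets it true, so the gate starts open.
; Box2 checks that flag before applying a velocity-change impulse through CharacterMovement.
; Both overlaps compare the player character to OverlappedComponent, the trigger's own component, rather than the other actor.
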(event OnComponentBeginOverlap(Box2)
  (params (OverlappedComponent :type Primitive%20Component%20Object%20Reference) (OtherActor :type Actor%20Object%20Reference) (OtherComp :type Primitive%20Component%20Object%20Reference) (OtherBodyIndex :type Integer) (bFromSweep :type Boolean) (SweepResult :type Hit%20Result%20Structure%20%28by%20ref%29))
  (if (Variables|Default|Get체크도달)
    (if (== (Game|GetPlayerCharacter 0) OverlappedComponent)
      (Physics|AddImpulse (Variables|/Script/Engine.Character|GetCharacterMovement (Game|GetPlayerCharacter 0)) "0.000000,0.000000,3000.000000" true))))

(event OnComponentBeginOverlap(Box)
  (params (OverlappedComponent :type Primitive%20Component%20Object%20Reference) (OtherActor :type Actor%20Object%20Reference) (OtherComp :type Primitive%20Component%20Object%20Reference) (OtherBodyIndex :type Integer) (bFromSweep :type Boolean) (SweepResult :type Hit%20Result%20Structure%20%28by%20ref%29))
  (if (== (Game|GetPlayerCharacter 0) OverlappedComponent)
    (Variables|Default|Set체크도달 true)))

(event EventBeginPlay
  (Variables|Default|Set체크도달 true))

(event Collision|EventActorBeginOverlap
  (params (OtherActor :type Actor%20Object%20Reference)))

(event EventTick
  (params (DeltaSeconds :type Float%20%28single-precision%29)))

(fn ConstructionScript)