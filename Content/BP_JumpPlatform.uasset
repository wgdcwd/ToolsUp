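; BP_JumpPlatform is a jump pad that launches the player character when an actor overlaps it.
; On overlap, 튀어오르기 applies a velocity-change impulse along the Arrow's forward vector, scaled by 점프력.
; 플레이어감지 compares the overlapping actor to the player but gates nothing, so any overlap triggers the launch.
; An optional ragdoll stun (조작막기) with delayed recovery to walking (일어나기) exists but is disconnected.
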(event EventBeginPlay)

(event Collision|EventActorBeginOverlap
  (params (OtherActor :type Actor%20Object%20Reference))
  (CallFunction|플레이어감지 OtherActor)
  (CallFunction|튀어오르기))

(event EventTick
  (params (DeltaSeconds :type Float%20%28single-precision%29)))

(fn ConstructionScript)

(fn 일어나기
  (Pawn|Components|CharacterMovement|SetMovementMode (Variables|/Script/Engine.Character|GetCharacterMovement (Game|GetPlayerCharacter 0)) "MOVE_Walking" 0))

(fn 튀어오르기
  (Physics|AddImpulse (Variables|/Script/Engine.Character|GetCharacterMovement (Game|GetPlayerCharacter 0)) (* (Math|Vector|GetForwardVector (Variables|Default|GetArrow)) (Variables|Default|Get점프력)) true))

(fn 플레이어감지
  (params (B :type Object%20Object%20Reference))
  (if (== (Game|GetPlayerCharacter 0) B)
    _))

(fn 조작막기
  (if (Variables|Default|Get기절)
    (Collision|SetCollisionProfileName (Variables|/Script/Engine.Character|GetMesh (Game|GetPlayerCharacter 0)) "Ragdoll" true :!class /Script/Engine.PrimitiveComponent)
    (Physics|SetSimulatePhysics (Variables|/Script/Engine.Character|GetMesh (Game|GetPlayerCharacter 0)) true)
    (Collision|SetCollisionEnabled (Variables|/Script/Engine.Character|GetMesh (Game|GetPlayerCharacter 0)) "NoCollision")
    (Pawn|Components|CharacterMovement|DisableMovement (Variables|/Script/Engine.Character|GetCharacterMovement (Game|GetPlayerCharacter 0)))))